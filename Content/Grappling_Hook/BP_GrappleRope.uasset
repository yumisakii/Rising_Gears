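; Grapple rope actor that draws a segmented rope mesh between a start and an end position.
; UpdateRope moves the two endpoints of a spline and lays fixed-length spline mesh segments along it.
; Segments come from a pool that grows on demand and hides surplus pieces instead of destroying them.
; The pool is sized before the endpoints move, so growth follows the spline length from the previous update.
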(event Custom|UpdateRope
  (params (StartPos :type Vector) (EndPos :type Vector))
  (bind _spline (Variables|Default|GetSpline))
  (bind _ropesegmentlength (Variables|Default|GetRopeSegmentLength))
  (bind _spline_2 (Variables|Default|GetSpline))
  (bind _ropesegmentlength_2 (Variables|Default|GetRopeSegmentLength))
  (bind _spline_3 (Variables|Default|GetSpline))
  (bind _ropepool (Variables|Default|GetRopePool))
  (bind _spline_4 (Variables|Default|GetSpline))
  (bind _returnvalue (Utilities|Array|Length _ropepool))
  (bind _returnvalue_2 (Spline|GetSplineLength _spline_2))
  (bind _returnvalue_3 (/ _returnvalue_2 _ropesegmentlength_2))
  (if (< _returnvalue _returnvalue_3)
    (for _index (range 1 (- _returnvalue_3 _returnvalue))
      (bind _returnvalue_4 (AddComponent|AddSplineMeshComponent false))
      (Transformation|SetMobility _returnvalue_4 "Movable")
      (Components|StaticMesh|SetStaticMesh _returnvalue_4 "/Game/Grappling_Hook/SM_Rope.SM_Rope")
      (Utilities|Array|Add (Variables|Default|GetRopePool) _returnvalue_4)))
  (Spline|SetLocationatSplinePoint _spline 0 StartPos "World" false)
  (Spline|SetLocationatSplinePoint _spline 1 EndPos "World" true)
  (for (_array_element _array_index) (Variables|Default|GetRopePool)
    (if (< _array_index (/ (Spline|GetSplineLength (Variables|Default|GetSpline)) (Variables|Default|GetRopeSegmentLength)))
      (Rendering|SetVisibility _array_element true false)
      (SplineMesh|SetStartandEnd _array_element (Spline|GetLocationatDistanceAlongSpline _spline_4 (Math|Conversions|ToFloat(Integer) (* _array_index _ropesegmentlength)) "Local") (* (Spline|GetDirectionatDistanceAlongSpline _spline_4 (Math|Conversions|ToFloat(Integer) (* _array_index _ropesegmentlength)) "Local") (Variables|Default|GetRopeSegmentLength)) (Spline|GetLocationatDistanceAlongSpline _spline_3 (Math|Conversions|ToFloat(Integer) (* (+ _array_index 1) _ropesegmentlength)) "Local") (* (Spline|GetDirectionatDistanceAlongSpline _spline_3 (Math|Conversions|ToFloat(Integer) (* (+ _array_index 1) _ropesegmentlength)) "Local") (Variables|Default|GetRopeSegmentLength)) true :!class /Script/Engine.SplineMeshComponent)
      (else
        (Rendering|SetVisibility _array_element false false)))))

(fn ConstructionScript)